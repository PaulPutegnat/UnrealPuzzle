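; Player controller that lets the player click tiles to set them moving.
; Left click runs a debug-drawn object line trace and calls ToggleMoving on any hit BP_Tile that is not already moving.
; The camera and control-rotation math in the trace endpoint helpers is left unconnected.
; The Pause input only casts the game mode to GM_Base, as its EventPause call never runs.
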(event `self.ReceiveBeginPlay`
  ;[1 0 0] Begin Play
  (`self.EnableInput` self))

(event `Trace`
  ;[0 1 0] Trace for tiles
  (bind _actortraced (`self.TraceTest` true))
  (if (`KismetSystemLibrary.IsValid` _actortraced)
    (bind _asbp_tile (cast `/Game/BP/BP_Tile` _actortraced))
    (if (not (`/Game/BP/BP_Tile.bIsMoving` _asbp_tile))
      (`/Game/BP/BP_Tile.ToggleMoving` _asbp_tile true))))

(event `Key|LeftMouseButton`
  (params (Key :type "Key Structure"))
  ;[0 1 0] Trace for tiles
  (:`Pressed`
    (`self.Trace`)))

(event `InputAction|Pause`
  (params (Key :type "Key Structure"))
  (:`Pressed`
    (bind _asgm_base (cast `/Game/BP/GM_Base` (`GameplayStatics.GetGameMode`)))))

(fn `TraceTest`
  (params (bDebug :type Boolean))
  (returns (ActorTraced :type "Actor Object Reference"))
  (bind _location (`self.GetStartLoc`))
  (bind _location_2 (`self.GetEndLoc` _location 12000.0))
  (if bDebug
    (`KismetSystemLibrary.DrawDebugLine` _location _location_2 (struct :`R` 1.0 :`A` 1.0) 0.1 1.0))
  (bind (_outhit _returnvalue) (`KismetSystemLibrary.LineTraceSingleForObjects` _location _location_2 (`|MakeArray` "ObjectTypeQuery1" "ObjectTypeQuery2" :!type "EObjectTypeQuery Enum") false (`|MakeArray` self (`GameplayStatics.GetPlayerPawn` 0) :!type "Actor Object Reference")))
  (bind (_bblockinghit _binitialoverlap _time _distance _location_3 _impactpoint _normal _impactnormal _physmat _hitactor) (`GameplayStatics.BreakHitResult` _outhit))
  (`KismetSystemLibrary.PrintString` (`KismetSystemLibrary.GetDisplayName` _hitactor))
  (if _returnvalue
    (return _hitactor)))

(fn `UserConstructionScript`)