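; Grid manager for a sliding-tile picture puzzle that builds, scrambles and checks the board.
; GeneratePuzzle spawns a grid of BP_Tile actors, slicing one texture across them through material offset and scale parameters, and records each home position.
; RandomizeTilesPosition removes the last tile to leave the empty slot, shuffles the rest and flags any already home.
; CheckWinCondition notifies GM_Base and shows W_Win once every tile is correctly placed.
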(event `self.ReceiveBeginPlay`
  (bind _returnvalue (`GameplayStatics.GetActorOfClass` "/Game/BP/GM_Base.GM_Base_C"))
  (set `self.GM_Base` _returnvalue))

(event `GeneratePuzzle`
  (params (NbLine :type Integer) (NbColumn :type Integer))
  (set `self.Nb Line` NbLine)
  (set `self.Nb Column` NbColumn)
  (set `self.Offset_X` (- (`self.Offset_X`) (`self.Step_X`)))
  (for _ (range 1 (+ (`self.Nb Column`) 1))
    (for _ (range 1 (+ (`self.Nb Line`) 1))
      (bind _output_get (set `self.Offset_X` (`KismetMathLibrary.FTrunc` (+ (`KismetMathLibrary.Conv_IntToDouble` (`self.Step_X`)) (`KismetMathLibrary.Conv_IntToDouble` (`self.Offset_X`))))))
      (bind _returnvalue (`|SpawnActorFromClass` "/Game/BP/BP_Tile.BP_Tile_C" (`KismetMathLibrary.MakeTransform` (+ (`KismetMathLibrary.MakeVector` (`KismetMathLibrary.Conv_IntToDouble` _output_get) (`KismetMathLibrary.Conv_IntToDouble` (`self.Offset_Y`))) (`self.K2_GetActorLocation`))) "Undefined" "OverrideRootScale" null null))
      (bind _material_instance (`/Game/BP/BP_Tile.Material_Instance` _returnvalue))
      (`MaterialInstanceDynamic.SetScalarParameterValue` _material_instance "OffsetX" (/ (/ (`KismetMathLibrary.Conv_IntToDouble` (`self.Offset_X`)) (`KismetMathLibrary.Conv_IntToDouble` (`self.Step_X`))) (`KismetMathLibrary.Conv_IntToDouble` (`self.Nb Line`))))
      (`MaterialInstanceDynamic.SetScalarParameterValue` _material_instance "OffsetY" (/ (/ (`KismetMathLibrary.Conv_IntToDouble` (`self.Offset_Y`)) (`KismetMathLibrary.Conv_IntToDouble` (`self.Step_Y`))) (`KismetMathLibrary.Conv_IntToDouble` (`self.Nb Column`))))
      (`MaterialInstanceDynamic.SetScalarParameterValue` _material_instance "ScaleX" (/ 1.0 (`KismetMathLibrary.Conv_IntToDouble` (`self.Nb Line`))))
      (`MaterialInstanceDynamic.SetScalarParameterValue` _material_instance "ScaleY" (/ 1.0 (`KismetMathLibrary.Conv_IntToDouble` (`self.Nb Column`))))
      (`MaterialInstanceDynamic.SetTextureParameterValue` _material_instance "TextureUsed" (`self.Texture`))
      (`/Engine/EditorBlueprintResources/StandardMacros.IncrementInt` (`self.Index`)
        (:`  `
          (bind _s_tiledata (make `/Game/Data/S_TileData` _returnvalue (`self.K2_GetActorLocation` _returnvalue) (1.0 1.0) (0.0 0.0)))
          (`KismetArrayLibrary.Array_Add` (`self.TileDataArray`) _s_tiledata)
          (set `/Game/BP/BP_Tile.TileData` _s_tiledata _returnvalue))))
    (set `self.Offset_X` (- 0 (`self.Step_X`)))
    (set `self.Offset_Y` (+ (`self.Offset_Y`) (`self.Step_Y`))))
  (`self.RandomizeTilesPosition`))

(fn `CheckWinCondition`
  (locals (PuzzleComplete :type Boolean :default true))
  (set `local.PuzzleComplete` true)
  (for _array_element (`self.TileDataArray`)
    (if (not (`.IsCorrectlyPlaced_20_819F4B9A4AF5C1F5108BE6A1E0A84350` (break `/Game/Data/S_TileData` _array_element)))
      (set `local.PuzzleComplete` false)
      (break)))
  (if (`local.PuzzleComplete`)
    (`/Game/BP/GM_Base.Event_Win` (`self.GM_Base`))
    (bind _returnvalue (`|CreateWidget` "/Game/UI/W_Win.W_Win_C"))
    (`UserWidget.AddToViewport` _returnvalue 0)))

(fn `RandomizeTilesPosition`
  (locals (`Randomized position` :type "Array of Vector Structure"))
  (bind _tiledataarray (`self.TileDataArray`))
  (bind _randomized_position (`local.Randomized position`))
  (bind _output (`|GetArrayItem` _tiledataarray (`KismetArrayLibrary.Array_LastIndex` _tiledataarray)))
  (bind (_tileactor _tileoriginalcoordinates) (break `/Game/Data/S_TileData` _output))
  ;[1 1 1] Destroy the bottom right tile and register it's position as empty
  (`self.K2_DestroyActor` _tileactor)
  (set `self.EmptyLocation` _tileoriginalcoordinates)
  (`KismetArrayLibrary.Array_RemoveItem` _tiledataarray _output)
  ;[1 1 1] Randomize each tile's position
  (for _array_element _tiledataarray
    (`KismetArrayLibrary.Array_Add` _randomized_position (`.Tileoriginalcoordinates_18_83F609CF4AEDC21AED4FFA9DD25F6DE1` (break `/Game/Data/S_TileData` _array_element))))
  (`KismetArrayLibrary.Array_Shuffle` _randomized_position)
  (for (_array_element_2 _array_index) _randomized_position
    (bind (_output_tileactor _output_tileoriginalcoordinates) (break `/Game/Data/S_TileData` (`|GetArrayItem` (`self.TileDataArray`) _array_index)))
    (`self.K2_SetActorLocation` _output_tileactor _array_element_2 false false)
    ;[1 1 1] Check if the tile is at it's original pos and if yes declare it
    (if (== _output_tileoriginalcoordinates _array_element_2 :`ErrorTolerance` 1.0)
      (bind (_output_tileactor_2 _output_tileoriginalcoordinates_2 _output_materialscale _output_materialoffset) (break `/Game/Data/S_TileData` (`|GetArrayItem` (`self.TileDataArray`) _array_index)))
      (bind _output_get (set `/Game/BP/BP_Tile.TileData` (make `/Game/Data/S_TileData` _output_tileactor_2 _output_tileoriginalcoordinates_2 _output_materialscale _output_materialoffset true) _output_tileactor_2))
      (`KismetArrayLibrary.Array_Set` (`self.TileDataArray`) _array_index _output_get))))

(fn `UserConstructionScript`)