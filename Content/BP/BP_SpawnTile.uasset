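; Spawns a grid of BP_Tile actors for a sliding picture puzzle, relative to this actor.
; GeneratePuzzle sets each tile's material to show its slice of one texture, recording positions in Bp_M_GridManager and tile data locally and on each tile.
; RandomizeTilesPosition then removes the last tile, registers its location as GM_Base's empty slot, and shuffles the others.
; SetTileMaterial returns zeroed scale and offset, so stored tile data lacks real UV values.
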(event `GeneratePuzzle`
  (params (NbLine :type Integer) (NbColumn :type Integer))
  (set `self.Nb Line` NbLine)
  (set `self.Nb Column` NbColumn)
  (bind _returnvalue (`GameplayStatics.GetActorOfClass` "/Game/BP/Bp_M_GridManager.Bp_M_GridManager_C"))
  (set `self.GridManager` _returnvalue)
  (set `self.Offset_X` (- (`self.Offset_X`) (`self.Step_X`)))
  (for _ (range 1 (+ (`self.Nb Column`) 1))
    (for _ (range 1 (+ (`self.Nb Line`) 1))
      (bind _output_get (set `self.Offset_X` (`KismetMathLibrary.FTrunc` (+ (`KismetMathLibrary.Conv_IntToDouble` (`self.Step_X`)) (`KismetMathLibrary.Conv_IntToDouble` (`self.Offset_X`))))))
      (bind _returnvalue_2 (`|SpawnActorFromClass` "/Game/BP/BP_Tile.BP_Tile_C" (`KismetMathLibrary.MakeTransform` (+ (`KismetMathLibrary.MakeVector` (`KismetMathLibrary.Conv_IntToDouble` _output_get) (`KismetMathLibrary.Conv_IntToDouble` (`self.Offset_Y`))) (`self.K2_GetActorLocation`))) "Undefined" "OverrideRootScale" null null))
      (bind _material_instance (`/Game/BP/BP_Tile.Material_Instance` _returnvalue_2))
      (`MaterialInstanceDynamic.SetScalarParameterValue` _material_instance "OffsetX" (/ (/ (`KismetMathLibrary.Conv_IntToDouble` (`self.Offset_X`)) (`KismetMathLibrary.Conv_IntToDouble` (`self.Step_X`))) (`KismetMathLibrary.Conv_IntToDouble` (`self.Nb Line`))))
      (`MaterialInstanceDynamic.SetScalarParameterValue` _material_instance "OffsetY" (/ (/ (`KismetMathLibrary.Conv_IntToDouble` (`self.Offset_Y`)) (`KismetMathLibrary.Conv_IntToDouble` (`self.Step_Y`))) (`KismetMathLibrary.Conv_IntToDouble` (`self.Nb Column`))))
      (`MaterialInstanceDynamic.SetScalarParameterValue` _material_instance "ScaleX" (/ 1.0 (`KismetMathLibrary.Conv_IntToDouble` (`self.Nb Line`))))
      (`MaterialInstanceDynamic.SetScalarParameterValue` _material_instance "ScaleY" (/ 1.0 (`KismetMathLibrary.Conv_IntToDouble` (`self.Nb Column`))))
      (`MaterialInstanceDynamic.SetTextureParameterValue` _material_instance "TextureUsed" (`self.Texture`))
      (bind _result (`/Engine/EditorBlueprintResources/StandardMacros.IncrementInt` (`self.Index`))
        (:`  `
          (bind _returnvalue_3 (`self.K2_GetActorLocation` _returnvalue_2))
          (`KismetArrayLibrary.Array_Set` (`/Game/BP/Bp_M_GridManager.TilesPosition` (`self.GridManager`)) _result _returnvalue_3 true)
          (bind _s_tiledata (make `/Game/Data/S_TileData` _returnvalue_2 _returnvalue_3 (1.0 1.0) (0.0 0.0)))
          (`KismetArrayLibrary.Array_Add` (`self.TileDataArray`) _s_tiledata)
          (set `/Game/BP/BP_Tile.TileData` _s_tiledata _returnvalue_2))))
    (set `self.Offset_X` (- 0 (`self.Step_X`)))
    (set `self.Offset_Y` (+ (`self.Offset_Y`) (`self.Step_Y`))))
  (`self.RandomizeTilesPosition`))

(fn `RandomizeTilesPosition`
  (locals (`Randomized position` :type "Array of Vector Structure"))
  (bind _tiledataarray (`self.TileDataArray`))
  (bind _randomized_position (`local.Randomized position`))
  (bind _output (`|GetArrayItem` _tiledataarray (`KismetArrayLibrary.Array_LastIndex` _tiledataarray)))
  (bind _tileactor (break `/Game/Data/S_TileData` _output))
  (`KismetSystemLibrary.PrintString` "Randomize (not implemented yet)")
  (bind _asgm_base (cast `/Game/BP/GM_Base` (`GameplayStatics.GetGameMode`)))
  (`/Game/BP/GM_Base.SetCurrentEmptyLoc` _asgm_base (`self.K2_GetActorLocation` _tileactor))
  (`self.K2_DestroyActor` _tileactor)
  (`KismetArrayLibrary.Array_RemoveItem` _tiledataarray _output)
  (for _array_element _tiledataarray
    (`KismetArrayLibrary.Array_Add` _randomized_position (`.Tileoriginalcoordinates_18_83F609CF4AEDC21AED4FFA9DD25F6DE1` (break `/Game/Data/S_TileData` _array_element))))
  (`KismetArrayLibrary.Array_Shuffle` _randomized_position)
  (for (_array_element_2 _array_index) _randomized_position
    (bind _output_tileactor (break `/Game/Data/S_TileData` (`|GetArrayItem` (`self.TileDataArray`) _array_index)))
    (`self.K2_SetActorLocation` _output_tileactor _array_element_2 false false)))

(fn `UserConstructionScript`)