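; GM_Base is a game mode Blueprint that creates the main HUD and tracks elapsed play time.
; BeginPlay clears the pause flag and adds a W_HUD widget to the viewport.
; Tick accumulates elapsed time while unpaused, and a pause event flips the flag and calls the CallEDPause dispatcher.
; The HUD's elapsed-time text update exists only as disconnected nodes.
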(event `self.ReceiveBeginPlay`
  (set `self.Pause` false)
  (bind _returnvalue (`|CreateWidget` "/Game/UI/W_HUD.W_HUD_C"))
  (bind _output_get (set `self.W_HUD` _returnvalue))
  (`UserWidget.AddToViewport` _output_get 0))

(event `self.ReceiveTick`
  (params (DeltaSeconds :type "Float (single-precision)"))
  (if (not (`self.Pause`))
    (set `self.ElapsedTime` (+ DeltaSeconds (`self.ElapsedTime`)))))

(event `Event_Pause`
  (set `self.Pause` (not (`self.Pause`)))
  (`self.ED_Pause`))

(fn `UserConstructionScript`)